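; BP_Projectile is a simple projectile actor built around a static mesh component.
; Launch applies a fixed impulse along the actor's forward vector as a velocity change, so the mesh's mass does not affect its speed.
; A component hit only prints a debug string, and a separate helper function prints the actor's display name.
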(event `self.StaticMeshComponent.OnComponentHit`
  (params (HitComponent :type "PrimitiveComponent Object Reference") (OtherActor :type "Actor Object Reference") (OtherComp :type "PrimitiveComponent Object Reference") (NormalImpulse :type "Vector Structure") (Hit :type "HitResult Structure (by ref)"))
  (`KismetSystemLibrary.PrintString` "yaaaah"))

(fn `Launch`
  (`PrimitiveComponent.AddImpulse` (`self.StaticMeshComponent`) (* (`self.GetActorForwardVector` self) 3000.0) "None" true))

(fn `Print your name`
  (`KismetSystemLibrary.PrintString` (`KismetSystemLibrary.GetDisplayName` self)))

(fn `UserConstructionScript`)